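; Pooled actor for Aurora's wall skill that computes spawn transforms for a ring of actors around the casting character.
; The PooledActorSetTransform event runs CalculationTransform, which casts SpawnInstigator to CharacterBase and appends to SpawnActorsTransform.
; Cosine and sine space ActorCount points evenly at Distance, offset by StartAngle plus the character's yaw, each facing inward toward the character.
; The spawning itself is not in these graphs.
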(event `self.BP_PooledActorSetTransform`
  (`self.CalculationTransform`))

(fn `CalculationTransform`
  (bind _actorcount (`self.ActorCount`))
  (bind _distance (`self.Distance`))
  (bind _ascharacter_base (cast `CharacterBase` (`self.SpawnInstigator`)))
  (for _index (range (`self.Index`) (+ _actorcount 1))
    (bind (_returnvalue_roll _returnvalue_pitch _returnvalue_yaw) (`KismetMathLibrary.BreakRotator` (`self.K2_GetActorRotation` _ascharacter_base)))
    (bind _returnvalue (+ (`KismetMathLibrary.MultiplyByPi` (* (/ (`KismetMathLibrary.Conv_IntToDouble` _index) (`KismetMathLibrary.Conv_IntToDouble` _actorcount)) (`KismetMathLibrary.Conv_IntToDouble` 2))) (`self.StartAngle`) (`KismetMathLibrary.DegreesToRadians` _returnvalue_yaw)))
    (bind _returnvalue_2 (`self.K2_GetActorLocation` _ascharacter_base))
    (bind _returnvalue_3 (+ (`KismetMathLibrary.MakeVector` (* _distance (`KismetMathLibrary.Cos` _returnvalue)) (* _distance (`KismetMathLibrary.Sin` _returnvalue))) _returnvalue_2))
    (`KismetArrayLibrary.Array_Add` (`self.SpawnActorsTransform`) (`KismetMathLibrary.MakeTransform` _returnvalue_3 (`KismetMathLibrary.MakeRotFromX` (- _returnvalue_2 _returnvalue_3))))))

(fn `UserConstructionScript`)